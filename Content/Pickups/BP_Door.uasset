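; BP_Door is a co-op exit check that tests whether players may open the door, currently only printing the result.
; When its Box is overlapped, the server checks that exactly two BP_ThirdPersonCharacter actors overlap the door.
; It then compares TotalCoins to MaxCoins in GS_Multiplayer_base and prints open, coins missing or not enough players.
; No door movement or state change is implemented.
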(event `self.Box.OnComponentBeginOverlap`
  (params (OverlappedComponent :type "PrimitiveComponent Object Reference") (OtherActor :type "Actor Object Reference") (OtherComp :type "PrimitiveComponent Object Reference") (OtherBodyIndex :type Integer) (bFromSweep :type Boolean) (SweepResult :type "HitResult Structure (by ref)"))
  (`/Engine/EditorBlueprintResources/ActorMacros.Switch Has Authority`
    (:`Authority`
      (if (== (`KismetArrayLibrary.Array_Length` (`self.GetOverlappingActors` "/Game/ThirdPerson/Blueprints/BP_ThirdPersonCharacter.BP_ThirdPersonCharacter_C")) 2)
        (bind _asgs_multiplayer_base (cast `/Game/ThirdPerson/Blueprints/GS_Multiplayer_base` (`GameplayStatics.GetGameState`)))
        (bind _maxcoins (`/Game/ThirdPerson/Blueprints/GS_Multiplayer_base.MaxCoins` _asgs_multiplayer_base))
        (if (== (`/Game/ThirdPerson/Blueprints/GS_Multiplayer_base.TotalCoins` _asgs_multiplayer_base) _maxcoins)
          (`KismetSystemLibrary.PrintString` "Door OPEN!")
          (else
            (`KismetSystemLibrary.PrintString` (`KismetStringLibrary.Concat_StrStr` "Not reached Max: " (`KismetStringLibrary.Conv_IntToString` _maxcoins)))))
        (else
          (`KismetSystemLibrary.PrintString` "Not enough players"))))))

(fn `UserConstructionScript`)